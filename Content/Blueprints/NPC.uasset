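; NPC character that wanders the navmesh at a random walk speed and can be talked to by the player.
; WalkEvent loops AIMoveTo to random reachable points within WalkRadius, pausing randomly after success or failure.
; TriggerArea overlaps set AIOverlap on the ThirdPersonCharacter and print greetings.
; TalkEvent halts movement and shows the Dialogue in AI_Dialogue_Widget; leaving the area restores speed and hides the widget.
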(event OnComponentBeginOverlap(TriggerArea)
  (params (OverlappedComponent :type Primitive%20Component%20Object%20Reference) (OtherActor :type Actor%20Object%20Reference) (OtherComp :type Primitive%20Component%20Object%20Reference) (OtherBodyIndex :type Integer) (bFromSweep :type Boolean) (SweepResult :type Hit%20Result%20Structure%20%28by%20ref%29))
  ;[1 1 1] Overlap Logic
  (bind _asthird_person_character (Utilities|Casting|CastToThirdPersonCharacter OtherActor))
  (Variables|/Game/ThirdPersonBP/Blueprints/ThirdPersonCharacter.ThirdPersonCharacter_C|SetAI%20Overlap _asthird_person_character true)
  (Development|PrintString " Hello there.."))

(event OnComponentEndOverlap(TriggerArea)
  (params (OverlappedComponent :type Primitive%20Component%20Object%20Reference) (OtherActor :type Actor%20Object%20Reference) (OtherComp :type Primitive%20Component%20Object%20Reference) (OtherBodyIndex :type Integer))
  ;[1 1 1] Overlap Logic
  (bind _asthird_person_character (Utilities|Casting|CastToThirdPersonCharacter OtherActor))
  (Variables|/Game/ThirdPersonBP/Blueprints/ThirdPersonCharacter.ThirdPersonCharacter_C|SetAI%20Overlap _asthird_person_character false)
  (Development|PrintString "Bye Bye mate")
  (Variables|Default|SetWalking? false)
  (Variables|/Script/Engine.CharacterMovementComponent|SetMaxWalkSpeed (Variables|Character|GetCharacterMovement) (Variables|Default|GetWalk_Speed))
  (Widget|SetVisibility (stale Custom|Talk%20Event _array_element) "Hidden"))

(event Custom|WalkEvent
  ;[1 1 1] NPC Walk Logic
  (if (not (Variables|Default|GetWalking?))
    (AI|AIMoveTo self (.RandomLocation (Class|NavigationSystemV1|GetRandomPointinNavigableRadius (Transformation|GetActorLocation) (Variables|Default|GetWalk_Radius) 0 0)) 0 5.0 false
      (:then
        (Variables|Default|SetWalking? true))
      (:OnSuccess
        (Utilities|FlowControl|Delay (Math|Random|RandomFloatinRange 1.0 5.0) :!label _label)
        (Variables|Default|SetWalking? false)
        (CallFunction|WalkEvent))
      (:OnFail
        (goto _label)))))

(event Custom|Talk%20Event
  ;[1 1 1] Interaction Dialogue Logic
  (Variables|/Script/Engine.CharacterMovementComponent|SetMaxWalkSpeed (Variables|Character|GetCharacterMovement) 0.0)
  (bind _foundwidgets (Widget|GetAllWidgetsOfClass "/Game/Blueprints/AI_Dialogue_Widget.AI_Dialogue_Widget_C" true))
  (for _array_element _foundwidgets
    (Variables|/Game/Blueprints/AI_Dialogue_Widget.AI_Dialogue_Widget_C|SetDialogue _array_element (Variables|Default|GetDialogue))
    (Widget|SetVisibility _array_element "Visible")))

(event EventBeginPlay
  ;[1 1 1] NPC Walk Logic
  (bind _output_get (Variables|Default|SetWalk_Speed (Math|Random|RandomFloatinRange 1e+02 4.5e+02)))
  (Variables|/Script/Engine.CharacterMovementComponent|SetMaxWalkSpeed (Variables|Character|GetCharacterMovement) _output_get)
  (CallFunction|WalkEvent))

(fn ConstructionScript)