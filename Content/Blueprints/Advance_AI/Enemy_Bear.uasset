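; Enemy bear character Blueprint that tracks health and dies when damage depletes it.
; AnyDamage subtracts truncated damage from CurrentHealth while it is above zero, then updates a health percentage and a display string.
; At zero or below, it clamps health, sets the string to "DEAD", plays a non-looping death animation directly on the mesh and disables movement.
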(event Game|Damage|EventAnyDamage
  (params (Damage :type Float%20%28single-precision%29) (DamageType :type Damage%20Type%20Object%20Reference) (InstigatedBy :type Controller%20Object%20Reference) (DamageCauser :type Actor%20Object%20Reference))
  ;[1 1 1] Receive damage
  (if (> (Variables|Default|GetCurrentHealth self) 0)
    (bind _output_get (Variables|Default|SetCurrentHealth (- (Variables|Default|GetCurrentHealth) (Math|Float|Truncate Damage))))
    (Variables|Default|SetHPPercent (/ (Math|Conversions|ToFloat(Integer) _output_get) (Math|Conversions|ToFloat(Integer) (Variables|Default|GetMaxHealth))))
    (Variables|Default|SetHPString (Utilities|String|ToString(Integer) _output_get))
    (if (<= _output_get 0)
      (Variables|Default|SetCurrentHealth 0)
      (Variables|Default|SetHPString "DEAD")
      (Components|Animation|PlayAnimation (Variables|Character|GetMesh) "/Game/InfinityBladeAdversaries/Enemy/Enemy_Bear/Enemy_Bear_Animations/ExoGame_Bears_Attack_Death.ExoGame_Bears_Attack_Death" false)
      (Pawn|Components|CharacterMovement|DisableMovement (Variables|Character|GetCharacterMovement)))))

(fn ConstructionScript
  (|CallParentFunction))