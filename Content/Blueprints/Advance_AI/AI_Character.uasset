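; AI enemy character with health, walk and chase speeds, and a timed hitscan attack on the player.
; Damage lowers health, updates the values for its overhead-style EnemyHPWidget, and destroys the actor at zero.
; StartAttack loops a FireWeapon timer that line traces to player 0 and applies fixed damage when it hits the ThirdPersonCharacter, until StopAttack clears it.
; Speed and attack events have no callers here.
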(event Custom|StopAttack
  ;[1 1 1] Attack Player
  (Utilities|Time|ClearTimerbyFunctionName 0 "Fire Weapon"))

(event Custom|StartAttack
  ;[1 1 1] Attack Player
  (Utilities|Time|SetTimerbyFunctionName 0 "Fire Weapon" (Variables|Default|GetAI%20Fire%20Rate) true))

(event Custom|ChaseSpeed
  ;[1 1 1] CharacterSpeed
  (Variables|/Script/Engine.CharacterMovementComponent|SetMaxWalkSpeed (Variables|Character|GetCharacterMovement) 4e+02))

(event Custom|Fire%20Weapon
  ;[1 1 1] Attack Player
  (Utilities|FlowControl|Sequence
    (:then_1
      (bind _outhit (Collision|LineTraceByChannel (Transformation|GetActorLocation) (Transformation|GetActorLocation (Game|GetPlayerCharacter 0)) "TraceTypeQuery1" false 0 "ForDuration"))
      (Utilities|FlowControl|Sequence
        (:then_0
          (bind _asthird_person_character (Utilities|Casting|CastToThirdPersonCharacter (.HitActor (Collision|BreakHitResult _outhit))))
          (Game|Damage|ApplyDamage _asthird_person_character 25.0 0 0)
          (Development|PrintString "Hitting Player"))
        (:then_1
          (Development|PrintString (Utilities|GetDisplayName (.HitActor (Collision|BreakHitResult _outhit)))))))))

(event Custom|WalkSpeed
  ;[1 1 1] CharacterSpeed
  (Variables|/Script/Engine.CharacterMovementComponent|SetMaxWalkSpeed (Variables|Character|GetCharacterMovement) 1e+02))

(event EventBeginPlay
  ;[1 1 1] Initialize character health on widget
  (bind _output_get (Variables|Default|SetCurrentHealth (Variables|Default|GetMaxHealth)))
  (Variables|Default|SetHPString (Utilities|String|ToString(Integer) _output_get))
  (bind _asenemy_hpwidget (Utilities|Casting|CastToEnemyHPWidget (UserInterface|GetUserWidgetObject (Variables|Default|GetEnemyWidget))))
  (Variables|/Game/UserInterface/EnemyHPWidget.EnemyHPWidget_C|SetEnemy _asenemy_hpwidget self))

(event Game|Damage|EventAnyDamage
  (params (Damage :type Float%20%28single-precision%29) (DamageType :type Damage%20Type%20Object%20Reference) (InstigatedBy :type Controller%20Object%20Reference) (DamageCauser :type Actor%20Object%20Reference))
  ;[1 1 1] Receive damage
  (bind _output_get (Variables|Default|SetCurrentHealth (- (Variables|Default|GetCurrentHealth) (Math|Float|Truncate Damage))))
  (Variables|Default|SetHPPercent (/ (Math|Conversions|ToFloat(Integer) _output_get) (Math|Conversions|ToFloat(Integer) (Variables|Default|GetMaxHealth))))
  (Variables|Default|SetHPString (Utilities|String|ToString(Integer) _output_get))
  (if (<= _output_get 0)
    (Actor|DestroyActor)
    (Development|PrintString "I'm dead")
    (else
      (Development|PrintString (Utilities|String|ToString(Integer) _output_get)))))

(fn ConstructionScript)