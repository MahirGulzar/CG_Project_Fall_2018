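; BP_NPC_Behaviour is an NPC that starts the BT_AdvanceAI behavior tree on BeginPlay, seeding TargetDestination with a random navigable point.
; Its trigger area sets AIOverlap on the ThirdPersonCharacter and prints greetings or farewells.
; TalkEvent stops movement and shows AI_Dialogue_Widget with its Dialogue; leaving restores WalkSpeed and hides the widget.
; The older random-speed AIMoveTo wander loop is disconnected, leaving WalkEvent empty.
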(event OnComponentBeginOverlap(TriggerArea)
  (params (OverlappedComponent :type Primitive%20Component%20Object%20Reference) (OtherActor :type Actor%20Object%20Reference) (OtherComp :type Primitive%20Component%20Object%20Reference) (OtherBodyIndex :type Integer) (bFromSweep :type Boolean) (SweepResult :type Hit%20Result%20Structure%20%28by%20ref%29))
  ;[1 1 1] Overlap Logic
  (bind _asthird_person_character (Utilities|Casting|CastToThirdPersonCharacter OtherActor))
  (Variables|/Game/Blueprints/ThirdPerson/ThirdPersonCharacter.ThirdPersonCharacter_C|SetAI%20Overlap _asthird_person_character true)
  (Development|PrintString " Hello there.."))

(event OnComponentEndOverlap(TriggerArea)
  (params (OverlappedComponent :type Primitive%20Component%20Object%20Reference) (OtherActor :type Actor%20Object%20Reference) (OtherComp :type Primitive%20Component%20Object%20Reference) (OtherBodyIndex :type Integer))
  ;[1 1 1] Overlap Logic
  (bind _asthird_person_character (Utilities|Casting|CastToThirdPersonCharacter OtherActor))
  (Variables|/Game/Blueprints/ThirdPerson/ThirdPersonCharacter.ThirdPersonCharacter_C|SetAI%20Overlap _asthird_person_character false)
  (Development|PrintString "Bye Bye mate")
  (Variables|Default|SetWalking? false)
  (Variables|/Script/Engine.CharacterMovementComponent|SetMaxWalkSpeed (Variables|Character|GetCharacterMovement) (Variables|Default|GetWalk_Speed))
  (Widget|SetVisibility (stale Custom|Talk%20Event _array_element) "Hidden"))

(event Custom|WalkEvent
  ;[1 1 1] NPC Walk Logic
)

(event Custom|Talk%20Event
  ;[1 1 1] Interaction Dialogue Logic
  (Variables|/Script/Engine.CharacterMovementComponent|SetMaxWalkSpeed (Variables|Character|GetCharacterMovement) 0.0)
  (bind _foundwidgets (Widget|GetAllWidgetsOfClass "/Game/Blueprints/AI_Dialogue_Widget.AI_Dialogue_Widget_C" true))
  (for _array_element _foundwidgets
    (Variables|/Game/Blueprints/AI_Dialogue_Widget.AI_Dialogue_Widget_C|SetDialogue _array_element (Variables|Default|GetDialogue))
    (Widget|SetVisibility _array_element "Visible")))

(event EventBeginPlay
  ;[1 1 1] NPC Walk Logic
  (AI|RunBehaviorTree (AI|GetAIController self) "/Game/Blueprints/Advance_AI/BT_AdvanceAI.BT_AdvanceAI")
  (AI|Components|Blackboard|SetValueasVector (AI|GetBlackboard self) (Utilities|Name|MakeLiteralName "TargetDestination") (.RandomLocation (Class|NavigationSystemV1|GetRandomPointinNavigableRadius (Transformation|GetActorLocation) (Variables|Default|GetWalk_Radius) 0 0))))

(fn ConstructionScript)