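; AI controller for AI_Character enemies that runs the BT_AdvanceAI behavior tree on possession.
; AI perception writes whether the ThirdPersonCharacter player is sensed to the CanSeePlayer Blackboard key; the follow-up sensed and lost branches only cast the pawn.
; Custom events forward walk speed, chase speed and attack start/stop requests to the controlled character.
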(event OnTargetPerceptionUpdated(AIPerception)
  (params (Actor :type Actor%20Object%20Reference) (Stimulus :type AI%20Stimulus%20Structure))
  (bind _bsuccessfullysensed (Utilities|Struct|BreakAIStimulus Stimulus))
  (bind _returnvalue (Pawn|GetControlledPawn))
  ;[1 1 1] AI perception on player sight
  (Utilities|Casting|CastToThirdPersonCharacter Actor)
  (AI|Components|Blackboard|SetValueasBool (AI|GetBlackboard 0) (Utilities|Name|MakeLiteralName "CanSeePlayer") _bsuccessfullysensed)
  (if _bsuccessfullysensed
    (Utilities|Casting|CastToAI_Character _returnvalue)
    (else
      (Utilities|Casting|CastToAI_Character _returnvalue))))

(event Custom|ChaseSpeed
  ;[1 1 1] Adjust AI speed w.r.t state
  (bind _asai_character (Utilities|Casting|CastToAI_Character (Pawn|GetControlledPawn)))
  (Default|ChaseSpeed _asai_character))

(event Custom|ObscuredSpeed
  ;[1 1 1] Adjust AI speed w.r.t state
  (bind _asai_character (Utilities|Casting|CastToAI_Character (Pawn|GetControlledPawn)))
  (Default|WalkSpeed _asai_character))

(event Custom|Stop%20AI%20Attack
  ;[1 1 1] Adjust AI speed w.r.t state
  (bind _asai_character (Utilities|Casting|CastToAI_Character (Pawn|GetControlledPawn)))
  (Default|StopAttack _asai_character))

(event Custom|Start%20AI%20Attack
  ;[1 1 1] Adjust AI speed w.r.t state
  (bind _asai_character (Utilities|Casting|CastToAI_Character (Pawn|GetControlledPawn)))
  (Default|StartAttack _asai_character))

(event EventOnPossess
  (params (PossessedPawn :type Pawn%20Object%20Reference))
  (Utilities|Casting|CastToAI_Character PossessedPawn)
  (AI|RunBehaviorTree "/Game/Blueprints/Advance_AI/BT_AdvanceAI.BT_AdvanceAI"))

(fn ConstructionScript)